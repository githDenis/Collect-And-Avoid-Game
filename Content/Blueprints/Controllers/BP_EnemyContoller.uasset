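; BP_EnemyContoller is an enemy AI controller that runs the BT_Enemy behavior tree on possession.
; On each perception update it plays a chase sound, writes the sensed state to the WasCharacterSeen blackboard key, and stores BP_Hero actors as MainCharacter.
; While no character is sensed, Tick writes a new random reachable point near the pawn to the RandomLoc key every frame.
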(event OnTargetPerceptionUpdated(AIPerception)
  (params (Actor :type Actor%20Object%20Reference) (Stimulus :type AI%20Stimulus%20Structure))
  (bind _output_get (Variables|Default|SetWasCharacterSeen (.bsuccessfullysensed Stimulus)))
  (Audio|PlaySound2D "/Game/Sounds/ChaseSound.ChaseSound" 1.0 1.0 0.0 0 0)
  (AI|Components|Blackboard|SetValueasBool (AI|GetBlackboard 0) (Utilities|Name|MakeLiteralName "WasCharacterSeen") _output_get)
  (bind _asbp_hero (Utilities|Casting|CastToBP_Hero Actor))
  (AI|Components|Blackboard|SetValueasObject (AI|GetBlackboard 0) (Utilities|Name|MakeLiteralName "MainCharacter") _asbp_hero))

(event EventBeginPlay)

(event EventTick
  (params (DeltaSeconds :type Float%20%28single-precision%29))
  (bind _returnvalue (Pawn|GetControlledPawn))
  (if (not (Variables|Default|GetWasCharacterSeen))
    (Utilities|IsValid _returnvalue
      (:Is%20Valid
        (AI|Components|Blackboard|SetValueasVector (AI|GetBlackboard 0) (Utilities|Name|MakeLiteralName "RandomLoc") (.RandomLocation (AI|Navigation|GetRandomReachablePointinRadius (Transformation|GetActorLocation _returnvalue) 6e+02 0 0)))))))

(event EventPossess
  (params (PossessedPawn :type Pawn%20Object%20Reference))
  (AI|RunBehaviorTree "/Game/AI/BT_Enemy.BT_Enemy"))

(fn ConstructionScript)