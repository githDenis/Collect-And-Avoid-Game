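; BP_Hero is the player character, using Enhanced Input for movement, look, jump, sprint and pause.
; Sprinting raises walk speed on player character 0 with a camera shake, while Tick drains stamina per frame and regenerates it otherwise.
; Running out of stamina restores walk speed but leaves IsSprinting set until sprint input ends, delaying regeneration.
; Pause toggles BP_MainHUD's PauseMenu, game pause, input mode and mouse cursor.
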(event Input|EnhancedActionEvents|EnhancedInputActionIA_MyJump
  (params (ActionValue :type Boolean) (ElapsedSeconds :type Float%20%28double-precision%29) (TriggeredSeconds :type Float%20%28double-precision%29) (InputAction :type Input%20Action%20Object%20Reference :default "/Game/Input/MyInput/IA_MyJump.IA_MyJump"))
  (:Triggered
    (Character|Jump))
  (:Completed
    (Character|StopJumping)))

(event Input|EnhancedActionEvents|EnhancedInputActionIA_Pause
  (params (ActionValue :type Boolean) (ElapsedSeconds :type Float%20%28double-precision%29) (TriggeredSeconds :type Float%20%28double-precision%29) (InputAction :type Input%20Action%20Object%20Reference :default "/Game/Input/MyInput/IA_Pause.IA_Pause"))
  (bind _returnvalue (Game|GetPlayerController 0))
  (:Started
    (bind _asbp_main_hud (Utilities|Casting|CastToBP_MainHUD (HUD|GetHUD (Game|GetPlayerController 0))))
    (Utilities|IsValid (Variables|/Game/UI/BP_MainHUD.BP_MainHUD_C|GetPauseMenu _asbp_main_hud)
      (:Is%20Valid
        (if (Game|IsGamePaused)
          (Widget|RemovefromParent (Variables|/Game/UI/BP_MainHUD.BP_MainHUD_C|GetPauseMenu _asbp_main_hud))
          (Input|SetInputModeGameOnly _returnvalue false)
          (Variables|/Script/Engine.PlayerController|SetbShowMouseCursor _returnvalue false)
          (Game|SetGamePaused false)
          (else
            (UserInterface|Viewport|AddtoViewport (Variables|/Game/UI/BP_MainHUD.BP_MainHUD_C|GetPauseMenu _asbp_main_hud) 0)
            (Input|SetInputModeGameandUI _returnvalue 0 "DoNotLock" true false)
            (Variables|/Script/Engine.PlayerController|SetbShowMouseCursor _returnvalue true)
            (Game|SetGamePaused true)))))))

(event Input|EnhancedActionEvents|EnhancedInputActionIA_MyMove
  (params (ActionValue :type Vector%202D%20Structure) (ElapsedSeconds :type Float%20%28double-precision%29) (TriggeredSeconds :type Float%20%28double-precision%29) (InputAction :type Input%20Action%20Object%20Reference :default "/Game/Input/MyInput/IA_MyMove.IA_MyMove"))
  (Pawn|Input|AddMovementInput (Transformation|GetActorForwardVector) (.y ActionValue) false)
  (Pawn|Input|AddMovementInput (Transformation|GetActorRightVector) (.x ActionValue) false))

(event Input|EnhancedActionEvents|EnhancedInputActionIA_MySprint
  (params (ActionValue :type Boolean) (ElapsedSeconds :type Float%20%28double-precision%29) (TriggeredSeconds :type Float%20%28double-precision%29) (InputAction :type Input%20Action%20Object%20Reference :default "/Game/Input/MyInput/IA_MySprint.IA_MySprint"))
  (:Started
    (if (!= (Variables|Default|GetIsSprinting) true)
      (Camera|PlayWorldCameraShake "/Game/Characters/CameraShake/BP_SprintShake.BP_SprintShake_C" (Transformation|GetActorLocation) 0.0 5e+02)
      (CallFunction|StartSprint)
      (Variables|Default|SetIsSprinting true)
      (else
        (CallFunction|StopSprint :!label _label)
        (Variables|Default|SetIsSprinting false))))
  (:Completed
    (goto _label)))

(event Input|EnhancedActionEvents|EnhancedInputActionIA_MyLook
  (params (ActionValue :type Vector%202D%20Structure) (ElapsedSeconds :type Float%20%28double-precision%29) (TriggeredSeconds :type Float%20%28double-precision%29) (InputAction :type Input%20Action%20Object%20Reference :default "/Game/Input/MyInput/IA_MyLook.IA_MyLook"))
  (Pawn|Input|AddControllerYawInput (.x ActionValue))
  (Pawn|Input|AddControllerPitchInput (.y ActionValue)))

(event EventBeginPlay
  (bind _returnvalue (Game|GetPlayerController 0))
  (bind _returnvalue_2 (PlayerController|LocalPlayerSubsystems|GetEnhancedInputLocalPlayerSubsystem _returnvalue))
  (Utilities|IsValid _returnvalue_2
    (:Is%20Valid
      (Input|AddMappingContext _returnvalue_2 "/Game/Input/MyInput/IMC_MyInput.IMC_MyInput" 0 "(bIgnoreAllPressedKeysUntilRelease=True,bForceImmediately=False,bNotifyUserSettings=False)"))))

(event Collision|EventActorBeginOverlap
  (params (OtherActor :type Actor%20Object%20Reference)))

(event EventTick
  (params (DeltaSeconds :type Float%20%28single-precision%29))
  (if (Variables|Default|GetIsSprinting)
    (if (> (Variables|Default|GetStamina) 0.0)
      (Variables|Default|SetStamina (- (Variables|Default|GetStamina) (Variables|Default|GetStaminaStep)))
      (else
        (CallFunction|StopSprint)))
    (elif (< (Variables|Default|GetStamina) (Variables|Default|GetMaxStamina))
      (Variables|Default|SetStamina (+ (Variables|Default|GetStamina) (Variables|Default|GetStaminaStep))))))

(fn ConstructionScript)

(fn StartSprint
  (bind _asbp_hero (Utilities|Casting|CastToBP_Hero (Game|GetPlayerCharacter 0)))
  (Variables|/Script/Engine.CharacterMovementComponent|SetMaxWalkSpeed (Variables|/Script/Engine.Character|GetCharacterMovement _asbp_hero) 1.2e+03))

(fn StopSprint
  (bind _asbp_hero (Utilities|Casting|CastToBP_Hero (Game|GetPlayerCharacter 0)))
  (Variables|/Script/Engine.CharacterMovementComponent|SetMaxWalkSpeed (Variables|/Script/Engine.Character|GetCharacterMovement _asbp_hero) 6e+02))