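; Game mode that tracks the player's score against a target and handles the win condition.
; Tick and IncreaseScore both derive the game state enum by comparing Score to TargetScore.
; IncreaseScore also pushes the new score to BP_MainHUD and, on reaching the target, pauses the game and shows the won screen.
; Helper functions set the game state directly or reset the score to zero.
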(event EventBeginPlay)

(event EventTick
  (params (DeltaSeconds :type Float%20%28single-precision%29))
  (if (< (Variables|Default|GetScore) (Variables|Default|GetTargetScore))
    (Variables|Default|SetCurrent%20Game%20State "NewEnumerator0")
    (else
      (Variables|Default|SetCurrent%20Game%20State "NewEnumerator1"))))

(fn ConstructionScript)

(fn SetCurrentGameState
  (params (Game%20State :type E_GameState%20Enum :default "NewEnumerator0"))
  (Variables|Default|SetCurrent%20Game%20State Game%20State))

(fn IncreaseScore
  (bind _output_get (Variables|Default|SetScore (+ (Variables|Default|GetScore) 1)))
  (if (< (Variables|Default|GetScore) (Variables|Default|GetTargetScore))
    (Variables|Default|SetCurrent%20Game%20State "NewEnumerator0")
    (else
      (Variables|Default|SetCurrent%20Game%20State "NewEnumerator1")))
  (bind _asbp_main_hud (Utilities|Casting|CastToBP_MainHUD (HUD|GetHUD (Game|GetPlayerController 0))))
  (Default|UpdateScore _asbp_main_hud _output_get)
  (if (== (Variables|Default|GetCurrent%20Game%20State) 1)
    (Game|SetGamePaused true)
    (Default|ShowWonScreen _asbp_main_hud)))

(fn ResetScore
  (Variables|Default|SetScore 0))